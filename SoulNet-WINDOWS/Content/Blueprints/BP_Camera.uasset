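; Shared multiplayer camera actor that frames all active players and eases back to a default position after they have been inactive for a set time.
; UpdatePosition interpolates the camera to the players' average location, pulled back along the Arrow's forward axis.
; Distance comes from the players' bounding box fitted to horizontal and vertical FOV, with a buffer and clamps.
; GetViewBounds derives visible extents from that distance.
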(event EventBeginPlay
  (bind _asbp_game_instance (Utilities|Casting|CastToBP_GameInstance (Game|GetGameInstance)))
  (Variables|Default|SetGameInstance _asbp_game_instance)
  (Utilities|CalculateVFOV))

(event Collision|EventActorBeginOverlap
  (params (OtherActor :type Actor%20Object%20Reference)))

(event EventTick
  (params (DeltaSeconds :type Float%20%28single-precision%29)))

(fn ConstructionScript)

(fn UpdatePosition
  (params (Players :type Array%20of%20BP%20Player%20Object%20References) (Last%20Active%20Player%20Time :type Float%20%28double-precision%29))
  (bind _returnvalue (Transformation|GetActorLocation))
  (if (Default|HasActivePlayers (Variables|Default|GetGameInstance) Players)
    (State|UpdateCameraDistance Players)
    (Transformation|SetActorLocation (Math|Interpolation|VInterpTo (Transformation|GetActorLocation) (Utilities|GetNextTargetLocation Players) (Utilities|Time|GetWorldDeltaSeconds) 1e+01) false false)
    (elif (and (> (- (Utilities|Time|GetGameTimeinSeconds) Last%20Active%20Player%20Time) (Variables|Default|GetTime%20To%20Reset%20Camera%20When%20Inactive)) (and (!= (.x _returnvalue) 0.0) (!= (.y _returnvalue) 0.0)))
      (Transformation|SetActorLocation (Math|Interpolation|VInterpTo (Transformation|GetActorLocation) (Math|Vector|MakeVector 0.0 0.0 (* (Variables|Default|GetMin%20Distance) -1.0)) (Utilities|Time|GetWorldDeltaSeconds) 2.0) false false)
      (Development|PrintString "RESET CAMERA"))))

(fn GetAverageActivePlayerLocation
  (params (%20Players :type Array%20of%20BP%20Player%20Object%20References))
  (bind _gameinstance (Variables|Default|GetGameInstance))
  (bind _active_players (Default|GetActivePlayers _gameinstance %20Players))
  (bind _returnvalue (Utilities|Array|Length _active_players))
  (if (Math|Conversions|ToBoolean(Integer) _returnvalue)
    (for _array_element _active_players
      (LocalVariables|SetPlayer%20Position%20Sum (+ (LocalVariables|GetPlayer%20Position%20Sum) (Transformation|GetActorLocation _array_element))))
    (return (Math|Vector|MakeVector (.x (/ (LocalVariables|GetPlayer%20Position%20Sum) _returnvalue)) (.y (/ (LocalVariables|GetPlayer%20Position%20Sum) _returnvalue)) 0.0))
    (else
      (return (LocalVariables|GetPlayer%20Position%20Sum)))))

(fn GetFurthestActivePlayerLocation
  (params (Players :type Array%20of%20BP%20Player%20Object%20References))
  (for _array_element (Default|GetActivePlayers (Variables|Default|GetGameInstance) Players)
    (if (> (Math|Float|Absolute(Float) (Math|Vector|VectorLength (- (Transformation|GetActorLocation _array_element) (Transformation|GetActorLocation)))) (LocalVariables|GetMost%20Distant%20Actor%20Distance))
      (LocalVariables|SetMost%20Distant%20Actor%20Distance (Math|Float|Absolute(Float) (Math|Vector|VectorLength (- (Transformation|GetActorLocation _array_element) (Transformation|GetActorLocation)))))
      (LocalVariables|SetMost%20Distant%20Actor%20Position (Transformation|GetActorLocation _array_element))))
  (return (LocalVariables|GetMost%20Distant%20Actor%20Position)))

(fn UpdateCameraDistance
  (params (Players :type Array%20of%20BP%20Player%20Object%20References))
  (if (== (Default|GetActivePlayersCount (Variables|Default|GetGameInstance) Players) 1)
    (Variables|Default|SetCamera%20Distance (Variables|Default|GetMin%20Distance))
    (else
      (bind _boxextent (Collision|GetActorArrayBounds (Default|GetActivePlayers (Variables|Default|GetGameInstance) Players) true))
      (Variables|Default|SetCamera%20Distance (Math|Float|Clamp(Float) (* (Math|Float|Max(Float) (/ (.x _boxextent) (Math|Trig|Tan(Degrees) (* (Variables|/Script/Engine.CameraComponent|GetFieldOfView (Variables|CameraActor|GetCameraComponent)) 0.5))) (/ (.y _boxextent) (Math|Trig|Tan(Degrees) (* (Variables|Default|GetVFOV) 0.5)))) (Variables|Default|GetDistance%20Buffer%20Size)) (Variables|Default|GetMin%20Distance) (Variables|Default|GetMax%20Distance))))))

(fn GetNextTargetLocation
  (params (%20Players :type Array%20of%20BP%20Player%20Object%20References))
  (return (+ (Utilities|GetAverageActivePlayerLocation %20Players) (* (Variables|Default|GetCamera%20Distance) (* -1.0 (Math|Vector|GetForwardVector (Variables|Default|GetArrow)))))))

(fn GetViewBounds
  (bind _returnvalue (Transformation|GetActorLocation))
  (bind _camera_distance (Variables|Default|GetCamera%20Distance))
  (bind _vfov (Variables|Default|GetVFOV))
  (bind _returnvalue_2 (* _vfov 0.5))
  (bind _returnvalue_3 (Math|Trig|Tan(Degrees) _returnvalue_2))
  (bind _returnvalue_4 (* _camera_distance _returnvalue_3))
  (bind _returnvalue_5 (* _returnvalue_4 1.0))
  (return (Class|KismetMathLibrary|MakeBoxSphereBounds (Math|Vector|MakeVector (.x _returnvalue) (.y _returnvalue) 0.0) (Math|Vector|MakeVector (* _returnvalue_5 (Variables|/Script/Engine.CameraComponent|GetAspectRatio (Variables|CameraActor|GetCameraComponent))) _returnvalue_5 0.0) 0.0)))

(fn CalculateVFOV
  (bind _output_get (Variables|Default|SetVFOV (* (Class|KismetMathLibrary|DegAtan (* (Math|Trig|Tan(Degrees) (* (Variables|/Script/Engine.CameraComponent|GetFieldOfView (Variables|CameraActor|GetCameraComponent)) 0.5)) (/ 1.0 (Variables|/Script/Engine.CameraComponent|GetAspectRatio (Variables|CameraActor|GetCameraComponent))))) 2.0)))
  (Development|PrintString (Utilities|String|ToString(Float) _output_get)))

(fn Initialize
  (Transformation|SetActorLocation (Math|Vector|MakeVector 0.0 0.0 (* (Variables|Default|GetMin%20Distance) -1.0)) false false)
  (Development|PrintString "CAMERA INSTANTIATED"))