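; Three-player actor with coloured physics spheres that move by input force and flock together, with player one's engagement and movement read from GameInstance_BP.
; Each Tick, nearby pairs share weighted input for alignment and attract each other beyond a minimum distance.
; A spring arm eases toward the active spheres' summed position divided by player count, while out-of-bounds spheres are pushed back toward it.
; Overlapping Trail-tagged actors destroys them and lengthens that sphere's Niagara trail.
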(event OnComponentBeginOverlap(Sphere1)
  (params (OverlappedComponent :type Primitive%20Component%20Object%20Reference) (OtherActor :type Actor%20Object%20Reference) (OtherComp :type Primitive%20Component%20Object%20Reference) (OtherBodyIndex :type Integer) (bFromSweep :type Boolean) (SweepResult :type Hit%20Result%20Structure%20%28by%20ref%29))
  (if (== OtherComp (Variables|Default|GetBoundaries))
    (Variables|Default|SetbOutOfBounds1 false)
    (else
      ;[1 1 1] Absorb trail
      (if (Actor|ActorHasTag OtherActor "Trail")
        (Niagara|SetNiagaraVariable(Float) (Variables|Default|GetNS_Trail1) "User.TrailLength" (+ (Variables|Default|GetTrailLength1) 0.1))
        (Variables|Default|SetTrailLength1 (+ (Variables|Default|GetTrailLength1) 0.1))
        (Actor|DestroyActor OtherActor)))))

(event OnComponentBeginOverlap(Sphere2)
  (params (OverlappedComponent :type Primitive%20Component%20Object%20Reference) (OtherActor :type Actor%20Object%20Reference) (OtherComp :type Primitive%20Component%20Object%20Reference) (OtherBodyIndex :type Integer) (bFromSweep :type Boolean) (SweepResult :type Hit%20Result%20Structure%20%28by%20ref%29))
  (if (== OtherComp (Variables|Default|GetBoundaries))
    (Variables|Default|SetbOutOfBounds2 false)
    (else
      ;[1 1 1] Absorb trail
      (if (Actor|ActorHasTag OtherActor "Trail")
        (Niagara|SetNiagaraVariable(Float) (Variables|Default|GetNS_Trail2) "User.TrailLength" (+ (Variables|Default|GetTrailLength2) 0.1))
        (Variables|Default|SetTrailLength2 (+ (Variables|Default|GetTrailLength2) 0.1))
        (Actor|DestroyActor OtherActor)))))

(event OnComponentBeginOverlap(Sphere3)
  (params (OverlappedComponent :type Primitive%20Component%20Object%20Reference) (OtherActor :type Actor%20Object%20Reference) (OtherComp :type Primitive%20Component%20Object%20Reference) (OtherBodyIndex :type Integer) (bFromSweep :type Boolean) (SweepResult :type Hit%20Result%20Structure%20%28by%20ref%29))
  (if (== OtherComp (Variables|Default|GetBoundaries))
    (Variables|Default|SetbOutOfBounds3 false)
    (else
      ;[1 1 1] Absorb trail
      (if (Actor|ActorHasTag OtherActor "Trail")
        (Niagara|SetNiagaraVariable(Float) (Variables|Default|GetNS_Trail3) "User.TrailLength" (+ (Variables|Default|GetTrailLength3) 0.1))
        (Variables|Default|SetTrailLength3 (+ (Variables|Default|GetTrailLength3) 0.1))
        (Actor|DestroyActor OtherActor)))))

(event OnComponentEndOverlap(Sphere1)
  (params (OverlappedComponent :type Primitive%20Component%20Object%20Reference) (OtherActor :type Actor%20Object%20Reference) (OtherComp :type Primitive%20Component%20Object%20Reference) (OtherBodyIndex :type Integer))
  ;[1 1 1] Trigger out of bounds pulling
  (if (== OtherComp (Variables|Default|GetBoundaries))
    (Variables|Default|SetbOutOfBounds1 true)))

(event OnComponentEndOverlap(Sphere2)
  (params (OverlappedComponent :type Primitive%20Component%20Object%20Reference) (OtherActor :type Actor%20Object%20Reference) (OtherComp :type Primitive%20Component%20Object%20Reference) (OtherBodyIndex :type Integer))
  ;[1 1 1] Trigger out of bounds pulling
  (if (== OtherComp (Variables|Default|GetBoundaries))
    (Variables|Default|SetbOutOfBounds2 true)))

(event OnComponentEndOverlap(Sphere3)
  (params (OverlappedComponent :type Primitive%20Component%20Object%20Reference) (OtherActor :type Actor%20Object%20Reference) (OtherComp :type Primitive%20Component%20Object%20Reference) (OtherBodyIndex :type Integer))
  ;[1 1 1] Trigger out of bounds pulling
  (if (== OtherComp (Variables|Default|GetBoundaries))
    (Variables|Default|SetbOutOfBounds3 true)))

(event EventTick
  (params (DeltaSeconds :type Float%20%28single-precision%29))
  (bind _springarm (Variables|Default|GetSpringArm))
  (bind _activeplayers (Variables|Default|GetActivePlayers))
  (bind _sphere1 (Variables|Default|GetSphere1))
  (bind _returnvalue (Transformation|GetWorldLocation _sphere1))
  (bind _output_get (Variables|Default|SetbActive1 (Variables|/Game/Blueprints/GameInstance_BP.GameInstance_BP_C|GetPlayer%20A%20is%20Engaged (Variables|Default|GetGameInstance))))
  (if _output_get
    (Math|Integer|IncrementInt (Variables|Default|GetActivePlayers)
      (:%20%20
        (Transformation|SetWorldLocation _sphere1 (Math|Vector|MakeVector (.x _returnvalue) (.y _returnvalue) 0.0) false false)))
    (else
      (Math|Integer|DecrementInt (Variables|Default|GetActivePlayers)
        (:%20%20
          (Transformation|SetWorldLocation _sphere1 (Math|Vector|MakeVector (.x _returnvalue) (.y _returnvalue) -2e+03) false false)))))
  (if (Variables|Default|GetbActive1)
    (bind _asgame_instance_bp (Utilities|Casting|CastToGameInstance_BP (Game|GetGameInstance)))
    ;[1 1 1] Move on input
    (CallFunction|MoveSphereonInput (Variables|Default|GetSphere1) (Utilities|Array|Get(acopy) (Variables|/Game/Blueprints/GameInstance_BP.GameInstance_BP_C|GetPlayer%20A%20Input _asgame_instance_bp)) (Utilities|Array|Get(acopy) (Variables|/Game/Blueprints/GameInstance_BP.GameInstance_BP_C|GetPlayer%20A%20Input _asgame_instance_bp) 1) 1.0))
  (if (Variables|Default|GetbActive2)
    (CallFunction|MoveSphereonInput (Variables|Default|GetSphere2) (Input|AxisValues|GetP2_UpDown) (Input|AxisValues|GetP2_RightLeft) 1.0))
  (if (Variables|Default|GetbActive3)
    (CallFunction|MoveSphereonInput (Variables|Default|GetSphere3) (Input|AxisValues|GetP3_UpDown) (Input|AxisValues|GetP3_RightLeft) 1.0))
  ;[1 1 1] Check proximity
  (bind _output_get_2 (CallFunction|SetS1S2Distance))
  (if (< _output_get_2 (Variables|Default|GetMaxPullDistance))
    ;[1 1 1] Alignment
    (CallFunction|MoveSphereonInput (Variables|Default|GetSphere1) (Input|AxisValues|GetP2_UpDown) (Input|AxisValues|GetP2_RightLeft) (Variables|Default|GetAlignmentWeight))
    (CallFunction|MoveSphereonInput (Variables|Default|GetSphere2) (Input|AxisValues|GetP1_UpDown) (Input|AxisValues|GetP1_RightLeft) (Variables|Default|GetAlignmentWeight))
    (if (> (Variables|Default|GetS1S2Distance) (Variables|Default|GetMinPullDistance))
      ;[1 1 1] Cohesion + Separation
      (CallFunction|MutualPull (Variables|Default|GetSphere1) (Variables|Default|GetSphere2))))
  (bind _output_get_3 (CallFunction|SetS2S3Distance))
  (if (< _output_get_3 (Variables|Default|GetMaxPullDistance))
    (CallFunction|MoveSphereonInput (Variables|Default|GetSphere2) (Input|AxisValues|GetP3_UpDown) (Input|AxisValues|GetP3_RightLeft) (Variables|Default|GetAlignmentWeight))
    (CallFunction|MoveSphereonInput (Variables|Default|GetSphere3) (Input|AxisValues|GetP2_UpDown) (Input|AxisValues|GetP2_RightLeft) (Variables|Default|GetAlignmentWeight))
    (if (> (Variables|Default|GetS2S3Distance) (Variables|Default|GetMinPullDistance))
      (CallFunction|MutualPull (Variables|Default|GetSphere2) (Variables|Default|GetSphere3))))
  (bind _output_get_4 (CallFunction|SetS3S1Distance))
  (if (< _output_get_4 (Variables|Default|GetMaxPullDistance))
    (CallFunction|MoveSphereonInput (Variables|Default|GetSphere3) (Input|AxisValues|GetP1_UpDown) (Input|AxisValues|GetP1_RightLeft) (Variables|Default|GetAlignmentWeight))
    (CallFunction|MoveSphereonInput (Variables|Default|GetSphere1) (Input|AxisValues|GetP3_UpDown) (Input|AxisValues|GetP3_RightLeft) (Variables|Default|GetAlignmentWeight))
    (if (> (Variables|Default|GetS3S1Distance) (Variables|Default|GetMinPullDistance))
      (CallFunction|MutualPull (Variables|Default|GetSphere3) (Variables|Default|GetSphere1))))
  (if (Variables|Default|GetbActive1)
    (Variables|Default|SetCameraLocationTarget (+ (Transformation|GetWorldLocation (Variables|Default|GetSphere1)) (Variables|Default|GetCameraLocationTarget))))
  (if (Variables|Default|GetbActive2)
    (Variables|Default|SetCameraLocationTarget (+ (Transformation|GetWorldLocation (Variables|Default|GetSphere2)) (Variables|Default|GetCameraLocationTarget))))
  (if (Variables|Default|GetbActive3)
    (bind _output_get_5 (Variables|Default|SetCameraLocationTarget (+ (Transformation|GetWorldLocation (Variables|Default|GetSphere3)) (Variables|Default|GetCameraLocationTarget)))))
  (if (> _activeplayers 0)
    (Transformation|SetWorldLocation _springarm (Math|Interpolation|VInterpTo (Transformation|GetWorldLocation _springarm) (Math|Vector|MakeVector (.x (/ _output_get_5 _activeplayers)) (.y (/ _output_get_5 _activeplayers)) 0.0) DeltaSeconds 1.0) false false)
    (Variables|Default|SetCameraLocationTarget "0, 0, 0")
    ;[1 1 1] Pull sphere into boundaries
    (if (Variables|Default|GetbActive1)
      (if (Variables|Default|GetbOutOfBounds1)
        (Physics|AddForce (Variables|Default|GetSphere1) (* (Math|Vector|Normalize (- (Variables|/Script/Engine.SceneComponent|GetRelativeLocation (Variables|Default|GetSpringArm)) (Variables|/Script/Engine.SceneComponent|GetRelativeLocation (Variables|Default|GetSphere1)))) (Variables|Default|GetBoundaryForce)) "None" false)))
    (if (Variables|Default|GetbActive2)
      (if (Variables|Default|GetbOutOfBounds2)
        (Physics|AddForce (Variables|Default|GetSphere2) (* (Math|Vector|Normalize (- (Variables|/Script/Engine.SceneComponent|GetRelativeLocation (Variables|Default|GetSpringArm)) (Variables|/Script/Engine.SceneComponent|GetRelativeLocation (Variables|Default|GetSphere2)))) (Variables|Default|GetBoundaryForce)) "None" false)))
    (if (Variables|Default|GetbActive3)
      (if (Variables|Default|GetbOutOfBounds3)
        (Physics|AddForce (Variables|Default|GetSphere3) (* (Math|Vector|Normalize (- (Variables|/Script/Engine.SceneComponent|GetRelativeLocation (Variables|Default|GetSpringArm)) (Variables|/Script/Engine.SceneComponent|GetRelativeLocation (Variables|Default|GetSphere3)))) (Variables|Default|GetBoundaryForce)) "None" false)))))

(event EventBeginPlay
  ;[1 1 1] Initialise colours
  (bind _asgame_instance_bp (Utilities|Casting|CastToGameInstance_BP (Game|GetGameInstance)))
  (Variables|Default|SetGameInstance _asgame_instance_bp)
  (bind _returnvalue (Rendering|Material|CreateDynamicMaterialInstance (Variables|Default|GetSphere1) 0 "/Game/Materials/M_Sphere.M_Sphere" "None" :!class /Script/Engine.PrimitiveComponent))
  (Rendering|Material|SetVectorParameterValue _returnvalue "Colour" (Class|KismetMathLibrary|LinearColorRed) :!class /Script/Engine.MaterialInstanceDynamic)
  (bind _returnvalue_2 (Rendering|Material|CreateDynamicMaterialInstance (Variables|Default|GetSphere2) 0 "/Game/Materials/M_Sphere.M_Sphere" "None" :!class /Script/Engine.PrimitiveComponent))
  (Rendering|Material|SetVectorParameterValue _returnvalue_2 "Colour" (Class|KismetMathLibrary|LinearColorGreen) :!class /Script/Engine.MaterialInstanceDynamic)
  (bind _returnvalue_3 (Rendering|Material|CreateDynamicMaterialInstance (Variables|Default|GetSphere3) 0 "/Game/Materials/M_Sphere.M_Sphere" "None" :!class /Script/Engine.PrimitiveComponent))
  (Rendering|Material|SetVectorParameterValue _returnvalue_3 "Colour" (Class|KismetMathLibrary|LinearColorBlue) :!class /Script/Engine.MaterialInstanceDynamic))

(event Input|ActionEvents|InputActionP2_Detection
  (params (Key :type Key%20Structure :default "None"))
  (bind _sphere2 (Variables|Default|GetSphere2))
  (bind _returnvalue (Transformation|GetWorldLocation _sphere2))
  (:Pressed
    (Variables|Default|SetbActive2 true)
    (Math|Integer|IncrementInt (Variables|Default|GetActivePlayers)
      (:%20%20
        (Transformation|SetWorldLocation _sphere2 (Math|Vector|MakeVector (.x _returnvalue) (.y _returnvalue) 0.0) false false))))
  (:Released
    (Variables|Default|SetbActive2 false)
    (Math|Integer|DecrementInt (Variables|Default|GetActivePlayers)
      (:%20%20
        (Transformation|SetWorldLocation _sphere2 (Math|Vector|MakeVector (.x _returnvalue) (.y _returnvalue) -2e+03) false false)))))

(event Input|ActionEvents|InputActionP3_Detection
  (params (Key :type Key%20Structure :default "None"))
  (bind _sphere3 (Variables|Default|GetSphere3))
  (bind _returnvalue (Transformation|GetWorldLocation _sphere3))
  (:Pressed
    (Variables|Default|SetbActive3 true)
    (Math|Integer|IncrementInt (Variables|Default|GetActivePlayers)
      (:%20%20
        (Transformation|SetWorldLocation _sphere3 (Math|Vector|MakeVector (.x _returnvalue) (.y _returnvalue) 0.0) false false))))
  (:Released
    (Variables|Default|SetbActive3 false)
    (Math|Integer|DecrementInt (Variables|Default|GetActivePlayers)
      (:%20%20
        (Transformation|SetWorldLocation _sphere3 (Math|Vector|MakeVector (.x _returnvalue) (.y _returnvalue) -2e+03) false false)))))

(event Input|ActionEvents|InputActionP1_Detection
  (params (Key :type Key%20Structure :default "None"))
  (bind _sphere1 (Variables|Default|GetSphere1))
  (bind _returnvalue (Transformation|GetWorldLocation _sphere1))
  (:Pressed
    (Variables|Default|SetbActive1 true)
    (Math|Integer|IncrementInt (Variables|Default|GetActivePlayers)
      (:%20%20
        (Transformation|SetWorldLocation _sphere1 (Math|Vector|MakeVector (.x _returnvalue) (.y _returnvalue) 0.0) false false))))
  (:Released
    (Variables|Default|SetbActive1 false)
    (Math|Integer|DecrementInt (Variables|Default|GetActivePlayers)
      (:%20%20
        (Transformation|SetWorldLocation _sphere1 (Math|Vector|MakeVector (.x _returnvalue) (.y _returnvalue) -2e+03) false false)))))

(fn ConstructionScript)

(fn SetS1S2Distance
  (bind _output_get (Variables|Default|SetS1S2Distance (Math|Vector|Distance2D(Vector) (Variables|/Script/Engine.SceneComponent|GetRelativeLocation (Variables|Default|GetSphere1)) (Variables|/Script/Engine.SceneComponent|GetRelativeLocation (Variables|Default|GetSphere2)))))
  (return _output_get))

(fn SetS2S3Distance
  (bind _output_get (Variables|Default|SetS2S3Distance (Math|Vector|Distance2D(Vector) (Variables|/Script/Engine.SceneComponent|GetRelativeLocation (Variables|Default|GetSphere2)) (Variables|/Script/Engine.SceneComponent|GetRelativeLocation (Variables|Default|GetSphere3)))))
  (return _output_get))

(fn SetS3S1Distance
  (bind _output_get (Variables|Default|SetS3S1Distance (Math|Vector|Distance2D(Vector) (Variables|/Script/Engine.SceneComponent|GetRelativeLocation (Variables|Default|GetSphere3)) (Variables|/Script/Engine.SceneComponent|GetRelativeLocation (Variables|Default|GetSphere1)))))
  (return _output_get))

(fn MoveSphereonInput
  (params (Sphere :type Primitive%20Component%20Object%20Reference) (X :type Float%20%28double-precision%29) (Y :type Float%20%28double-precision%29) (ForceFactor :type Float%20%28double-precision%29))
  (Physics|AddForce Sphere (* (* (Math|Vector|Normalize (Math|Vector|MakeVector X Y 0.0)) (Variables|Default|GetSpeed)) ForceFactor) "None" false))

(fn MutualPull
  (params (Sphere :type Primitive%20Component%20Object%20Reference) (OtherSphere :type Primitive%20Component%20Object%20Reference))
  (Physics|AddForce Sphere (* (Math|Vector|Normalize (- (Variables|/Script/Engine.SceneComponent|GetRelativeLocation OtherSphere) (Variables|/Script/Engine.SceneComponent|GetRelativeLocation Sphere))) (Variables|Default|GetPullForce)) "None" false)
  (Physics|AddForce OtherSphere (* (Math|Vector|Normalize (- (Variables|/Script/Engine.SceneComponent|GetRelativeLocation Sphere) (Variables|/Script/Engine.SceneComponent|GetRelativeLocation OtherSphere))) (Variables|Default|GetPullForce)) "None" false))