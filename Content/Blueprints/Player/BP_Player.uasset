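; BP_Player is an indexed, coloured physics sphere player, pushed by input plus alignment, cohesion and inward flocking forces.
; UpdateState switches between standby, pre-active, active and disconnected, driving respawn near active players, death, visibility and Niagara effects.
; Overlaps lengthen its Niagara trail and trigger item audio.
; MetaSound triggers handle movement audio and queued narration, which dampens other players, while a random timer prints placeholder voice comments.
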(event Custom|Event%20InitialiseMaterial
  (params (PlayerIndex :type Integer))
  (Setup|InitialiseMaterial PlayerIndex))

(event Custom|OnFinishedAudio_Event
  (Audio|OnNarrativeAudioFinished))

(event EventBeginPlay
  (Utilities|FlowControl|Sequence
    (:then_0
      (Variables|State|SetbActive false)
      (bind _asbp_game_instance (Utilities|Casting|CastToBP_GameInstance (Game|GetGameInstance)))
      (Variables|State|SetBP%20Game%20Instance _asbp_game_instance))
    (:then_1
      (EventDispatchers|BindEventtoOnAudioFinished (Variables|Default|GetMS_PlayerNarrative) (delegate Custom|OnFinishedAudio_Event)))))

(event Collision|EventActorBeginOverlap
  (params (OtherActor :type Actor%20Object%20Reference))
  (Collisions|HandleTrailBeginOverlap OtherActor)
  (CallFunction|AbsorbTrail)
  (CallFunction|TriggerItemAudio))

(event EventTick
  (params (DeltaSeconds :type Float%20%28single-precision%29))
  (if (Variables|State|GetbActive)
    (Utilities|FlowControl|Sequence
      (:then_0
        (Update|MoveSphere)
        (CallFunction|HandleMovementAudio))
      (:then_1
        (Update|ResetVectors)))))

(event Collision|EventActorEndOverlap
  (params (OtherActor :type Actor%20Object%20Reference))
  ;[1 1 1] Delete?
)

(fn ConstructionScript)

(fn Initialize
  (params (Player%20Index :type Integer))
  (Variables|State|SetPlayer%20Index Player%20Index)
  (Components|Activation|SetActive (Variables|Default|GetTrail) false false)
  (Transformation|SetActorLocation (Math|Vector|MakeVector (Math|Random|RandomFloatinRange -5e+02 5e+02) (Math|Random|RandomFloatinRange -5e+02 5e+02) 0.0) false false)
  (Setup|InitialiseMaterial Player%20Index)
  (Collision|SetActorEnableCollision false)
  (Actor|Tick|SetActorTickEnabled false)
  (Rendering|SetActorHiddenInGame true)
  (Effects|Components|ParticleSystem|SetIntParameter (Variables|Default|GetMS_PlayerNarrative) "Player Index" (Variables|State|GetPlayer%20Index))
  (Development|PrintString (Utilities|String|Append "Player " (Utilities|String|ToString(Integer) (Variables|State|GetPlayer%20Index)) " spawned"))
  (Development|PrintString (Utilities|String|ToString(Vector) (Transformation|GetActorLocation)) true true "(R=0.000000,G=1.000000,B=0.134609,A=1.000000)"))

(fn InitialiseMaterial
  (params (Player%20Index :type Integer))
  (bind _returnvalue (Rendering|Material|CreateDynamicMaterialInstance (Variables|Default|GetSphere) 0 (Utilities|Array|Get(acopy) (Variables|Appearence|GetMatArray) (Variables|State|GetPlayer%20Index)) "None" :!class /Script/Engine.PrimitiveComponent))
  (Rendering|Material|SetVectorParameterValue _returnvalue "Colour" (Utilities|Array|Get(acopy) (Variables|Appearence|GetSphereColours) Player%20Index) :!class /Script/Engine.MaterialInstanceDynamic))

(fn HandleBoundaryEndOverlap
  (params (OtherActor :type Actor%20Object%20Reference))
  (if (Actor|ActorHasTag OtherActor "Boundaries")
    (Variables|State|SetbOutOfBounds true)))

(fn HandleTrailBeginOverlap
  (params (OtherActor :type Actor%20Object%20Reference))
  (Utilities|Casting|CastToBP_ItemA OtherActor
    (:then
      (Development|PrintString (Utilities|String|Append (Utilities|GetDisplayName self) " COLLIDED") :!label _label))
    (:CastFailed
      (Utilities|Casting|CastToBP_ItemB OtherActor
        (:then
          (goto _label))
        (:CastFailed
          (Utilities|Casting|CastToBP_ItemC OtherActor
            (:then
              (goto _label))
            (:CastFailed
              (Utilities|Casting|CastToBP_ItemD OtherActor
                (:then
                  (goto _label))
                (:CastFailed
                  (Development|PrintString "COLLISION NOT RECOGNISED"))))))))))

(fn HandleBoundaryBeginOverlap
  (params (Other%20Actor :type Actor%20Object%20Reference))
  (if (Actor|ActorHasTag Other%20Actor "Boundaries")
    (Variables|State|SetbOutOfBounds false)
    (Development|PrintString "Hello")))

(fn UpdateOutOfBounds
  (params (View%20Bounds :type Box%20Sphere%20Bounds%20Structure))
  ;[1 1 1] TODO: fix out of bounds bug
  (Variables|State|SetbOutOfBounds (Utilties|IsinViewBounds View%20Bounds)))

(fn MoveSphere
  (if (Utilities|Enum|Equal(Enum) (Variables|State|GetCurrent%20State) "NewEnumerator2")
    (Physics|AddForce (Variables|Default|GetSphere) (+ (* (Variables|Motion|GetInputVector) (Variables|Motion|GetSpeed)) (* (Variables|Motion|GetAlignmentVector) (Variables|Motion|GetAlignmentWeight) (Variables|Motion|GetSpeed)) (* (Variables|Motion|GetCohesionVector) (Variables|Motion|GetCohesionWeight) (Variables|Motion|GetSpeed)) (* (Variables|Motion|GetInwardForceVector) (Variables|Motion|GetInwardForceWeight) (Variables|Motion|GetSpeed))) "None" false)))

(fn ResetVectors
  (Variables|Motion|SetAlignmentVector "0, 0, 0")
  (Variables|Motion|SetCohesionVector "0, 0, 0"))

(fn Respawn
  (params (Players :type Array%20of%20BP%20Player%20Object%20References) (Camera :type BP%20Camera%20Object%20Reference))
  (bind _trail (Variables|Default|GetTrail))
  (Variables|State|SetbActive true)
  (Transformation|SetActorLocation (Utilties|GetRespawnLocation Players Camera) false true)
  (Collision|SetActorEnableCollision true)
  (Actor|Tick|SetActorTickEnabled true)
  (Rendering|SetActorHiddenInGame false)
  (Development|PrintString (Utilities|String|Append "Player  active: " (Utilities|String|ToString(Integer) (Variables|State|GetPlayer%20Index))))
  (Components|Activation|SetActive _trail true false)
  (Niagara|ReinitializeSystem _trail)
  (bind _asaudio_parameter_controller_interface (Utilities|Casting|CastToAudioParameterControllerInterface (Variables|Default|GetPlayerAudio)))
  (Class|AudioParameterControllerInterface|SetTriggerParameter _asaudio_parameter_controller_interface "PlayIdle")
  ;[1 1 1] Trigger first comment after x seconds
  (bind _returnvalue (Utilities|Time|SetTimerbyFunctionName 0 "TriggerVoiceComment" (Math|Random|RandomFloatinRange 5.0 5e+01)))
  (Variables|State|SetCurrentTimer _returnvalue))

(fn IsinViewBounds
  (params (Bounds :type Box%20Sphere%20Bounds%20Structure))
  (bind _returnvalue (Transformation|GetActorLocation))
  (bind _bounds_shrink_factor (LocalVariables|GetBounds%20Shrink%20Factor))
  (bind _bounds_shrink_factor_2 (LocalVariables|GetBounds%20Shrink%20Factor))
  (bind _returnvalue_2 (- (.x _returnvalue) (.x (.origin Bounds))))
  (bind _returnvalue_3 (* (.x (.boxextent Bounds)) _bounds_shrink_factor_2))
  (bind _returnvalue_4 (* (.y (.boxextent Bounds)) _bounds_shrink_factor))
  (bind _returnvalue_5 (- (.y _returnvalue) (.y (.origin Bounds))))
  (bind _returnvalue_6 (Math|Float|Absolute(Float) _returnvalue_5))
  (bind _returnvalue_7 (Math|Float|Absolute(Float) _returnvalue_2))
  (bind _returnvalue_8 (> _returnvalue_7 _returnvalue_3))
  (bind _returnvalue_9 (> _returnvalue_6 _returnvalue_4))
  (bind _returnvalue_10 (or _returnvalue_8 _returnvalue_9))
  (if _returnvalue_10
    (Development|PrintString (Utilities|String|Append "Player Out of Bounds: " (Utilities|String|ToString(Integer) (Variables|State|GetPlayer%20Index))))
    (return _returnvalue_10)))

(fn Die
  (Collision|SetActorEnableCollision false)
  (Actor|Tick|SetActorTickEnabled false)
  (Development|SetHiddeninGame (Variables|Default|GetSphere) true false)
  (Development|PrintString (Utilities|String|Append "Player  inactive: " (Utilities|String|ToString(Integer) (Variables|State|GetPlayer%20Index))))
  (bind _output_get (Variables|Appearence|SetTrailLength 0.3))
  (Niagara|SetNiagaraVariable(Float) (Variables|Default|GetTrail) "User.TrailLength" _output_get)
  (Components|Activation|SetActive (Variables|Default|GetTrail) false false)
  (bind _asaudio_parameter_controller_interface (Utilities|Casting|CastToAudioParameterControllerInterface (Variables|Default|GetPlayerAudio)))
  (Class|AudioParameterControllerInterface|SetTriggerParameter _asaudio_parameter_controller_interface "StopIdle")
  (Utilities|Time|ClearandInvalidateTimerbyHandle (Variables|State|GetCurrentTimer)))

(fn GetRespawnLocation
  (params (Players :type Array%20of%20BP%20Player%20Object%20References) (Camera :type BP%20Camera%20Object%20Reference))
  (bind _returnvalue (Math|Random|RandomUnitVector))
  (bind _min_spawn_distance (LocalVariables|GetMin%20Spawn%20Distance))
  (bind _max_spawn_distance (LocalVariables|GetMax%20Spawn%20Distance))
  (bind _returnvalue_2 (Math|Random|RandomFloatinRange _min_spawn_distance _max_spawn_distance))
  (bind _returnvalue_3 (* _returnvalue _returnvalue_2))
  (if (CallFunction|IsPlayerinCameraBounds Camera)
    (return (Transformation|GetActorLocation))
    (else
      (bind _center (Collision|GetActorArrayBounds (Default|GetActivePlayers (Variables|State|GetBP%20Game%20Instance) Players) true))
      (return (+ _center (Math|Vector|MakeVector (.x _returnvalue_3) (.y _returnvalue_3) 0.0))))))

(fn HandleMovementAudio
  (bind _returnvalue (Transformation|GetVelocity))
  (bind _returnvalue_2 (Math|Vector|VectorIsNearlyZero _returnvalue 5e+01))
  (if (and (Variables|State|GetbMoving) _returnvalue_2)
    (bind _asaudio_parameter_controller_interface (Utilities|Casting|CastToAudioParameterControllerInterface (Variables|Default|GetPlayerAudio)))
    (Class|AudioParameterControllerInterface|SetTriggerParameter _asaudio_parameter_controller_interface "StopMoving")
    (Variables|State|SetbMoving false)
    (elif (Math|Boolean|NORBoolean _returnvalue_2 (Variables|State|GetbMoving))
      (bind _asaudio_parameter_controller_interface_2 (Utilities|Casting|CastToAudioParameterControllerInterface (Variables|Default|GetPlayerAudio)))
      (Class|AudioParameterControllerInterface|SetTriggerParameter _asaudio_parameter_controller_interface_2 "PlayMoving")
      (Variables|State|SetbMoving true))))

(fn TriggerItemAudio
  (bind _asaudio_parameter_controller_interface (Utilities|Casting|CastToAudioParameterControllerInterface (Variables|Default|GetItemAudio)))
  (Class|AudioParameterControllerInterface|SetTriggerParameter _asaudio_parameter_controller_interface "Collide"))

(fn AbsorbTrail
  (Niagara|SetNiagaraVariable(Float) (Variables|Default|GetTrail) "User.TrailLength" (+ (Variables|Appearence|GetTrailLength) 0.1))
  (Variables|Appearence|SetTrailLength (+ (Variables|Appearence|GetTrailLength) 0.1)))

(fn TriggerVoiceComment
  (if (Variables|State|GetbActive)
    (Development|PrintString (Utilities|String|Append "PLAYER " (Utilities|String|ToString(Integer) (Variables|State|GetPlayer%20Index)) ", TRY TO RELAX, YOUR BIOMETRICS ARE SUBOPTIMAL") true true "(R=1.000000,G=0.000000,B=1.000000,A=1.000000)" 3.0)
    (bind _returnvalue (Utilities|Time|SetTimerbyFunctionName 0 "TriggerVoiceComment" (Math|Random|RandomFloatinRange 5.0 5e+01)))
    (Variables|State|SetCurrentTimer _returnvalue)))

(fn UpdateState
  (params (Player%20State :type ENUM_PlayerState%20Enum :default "NewEnumerator0") (Players :type Array%20of%20BP%20Player%20Object%20References) (Camera :type BP%20Camera%20Object%20Reference))
  (if (Utilities|Enum|NotEqual(Enum) Player%20State (Variables|State|GetCurrent%20State))
    (LocalVariables|SetPrevious%20State (Variables|State|GetCurrent%20State))
    (Variables|State|SetCurrent%20State Player%20State)
    (Audio|ClearAudioQueue)
    (Development|PrintString (Utilities|String|Append "Player " (Utilities|String|ToString(Integer) (Variables|State|GetPlayer%20Index)) " state change: " (Utilities|String|EnumtoString (Variables|State|GetCurrent%20State))))
    (switch Utilities|FlowControl|Switch|SwitchonENUM_PlayerState (Variables|State|GetCurrent%20State)
      (:NewEnumerator0
        (StateChange|SetStanbyState (LocalVariables|GetPrevious%20State) Players))
      (:NewEnumerator1
        (StateChange|SetPreActiveState (LocalVariables|GetPrevious%20State) Players Camera))
      (:NewEnumerator2
        (StateChange|SetActiveState (LocalVariables|GetPrevious%20State) Players))
      (:NewEnumerator3
        (StateChange|SetDisconnectedState (LocalVariables|GetPrevious%20State) Players)))))

(fn SetStanbyState
  (params (Previous%20State :type ENUM_PlayerState%20Enum :default "NewEnumerator0") (Players :type Array%20of%20BP%20Player%20Object%20References))
  (Utilities|FlowControl|Sequence
    (:then_0
      (if (Utilities|Enum|Equal(Enum) Previous%20State "NewEnumerator3")
        (Development|SetHiddeninGame (Variables|Default|GetSphere) true false)
        (Components|Activation|Deactivate (Variables|Default|GetDisconnected%20Animation))
        (Audio|QueueAudio "Death")
        (Events|Die :!label _label)))
    (:then_1
      (if (Utilities|Enum|Equal(Enum) Previous%20State "NewEnumerator1")
        (Components|Activation|Deactivate (Variables|Default|GetActivationNiagara))
        (goto _label)))))

(fn SetPreActiveState
  (params (Previous%20State :type ENUM_PlayerState%20Enum :default "NewEnumerator0") (Players :type Array%20of%20BP%20Player%20Object%20References) (Camera :type BP%20Camera%20Object%20Reference))
  (bind _activationniagara (Variables|Default|GetActivationNiagara))
  (if (Utilities|Enum|Equal(Enum) Previous%20State "NewEnumerator0")
    (Events|Respawn Players Camera)
    (Development|SetHiddeninGame (Variables|Default|GetSphere) true false)
    (Niagara|ResetSystem _activationniagara)
    (Niagara|ReinitializeSystem _activationniagara)
    (Components|Activation|Activate _activationniagara false)
    (Audio|QueueAudio "PreActive")))

(fn SetActiveState
  (params (Previous%20State :type ENUM_PlayerState%20Enum :default "NewEnumerator0") (Players :type Array%20of%20BP%20Player%20Object%20References))
  (Utilities|FlowControl|Sequence
    (:then_0
      (if (Utilities|Enum|Equal(Enum) Previous%20State "NewEnumerator3")
        (Components|Activation|Deactivate (Variables|Default|GetDisconnected%20Animation))
        (Development|SetHiddeninGame (Variables|Default|GetSphere) false false :!label _label)))
    (:then_1
      (if (Utilities|Enum|Equal(Enum) Previous%20State "NewEnumerator1")
        (Components|Activation|Deactivate (Variables|Default|GetActivationNiagara))
        (Audio|QueueAudio "Active")
        (goto _label)))))

(fn SetDisconnectedState
  (params (Previous%20State :type ENUM_PlayerState%20Enum :default "NewEnumerator0") (Players :type Array%20of%20BP%20Player%20Object%20References))
  (if (Utilities|Enum|Equal(Enum) Previous%20State "NewEnumerator2")
    (Niagara|ReinitializeSystem (Variables|Default|GetDisconnected%20Animation))
    (Components|Activation|Activate (Variables|Default|GetDisconnected%20Animation) false)
    (Variables|Appearence|SetTrailLength 0.0)
    (Audio|QueueAudio "Disconnected Message1")))

(fn IsPlayerinCameraBounds
  (params (Camera :type BP%20Camera%20Object%20Reference))
  (return (Default|IsPositioninBoxBounds (Variables|State|GetBP%20Game%20Instance) (Default|GetViewBounds Camera) (Transformation|GetActorLocation) 1e+02)))

(fn PlaySoundforPlayer
  (params (Trigger%20Name :type Name) (Force%20Play :type Boolean))
  (bind _ms_playernarrative (Variables|Default|GetMS_PlayerNarrative))
  (if (or Force%20Play (not (Variables|Sound|GetIs%20Audio%20Playing)))
    (Variables|Sound|SetIs%20Audio%20Playing true)
    (Audio|Components|Audio|Play _ms_playernarrative 0.0)
    (Class|AudioParameterControllerInterface|SetTriggerParameter _ms_playernarrative Trigger%20Name)))

(fn PlayQueudAudio
  (params (Players :type Array%20of%20BP%20Player%20Object%20References))
  (if (or (== (Utilities|Array|Length (Variables|Sound|GetAudio%20Queue)) 0) (Variables|Sound|GetIs%20Audio%20Playing))
    (return)
    (else
      (Audio|PlaySoundforPlayer (Utilities|Array|Get(acopy) (Variables|Sound|GetAudio%20Queue)) false)
      (Utilities|Array|RemoveIndex (Variables|Sound|GetAudio%20Queue))
      ;[1 1 1] Dampen other playing audio
      (for _array_element Players
        (if (!= _array_element self)
          (Audio|DampenPlayingAudio _array_element))))))

(fn DampenPlayingAudio
  (Class|AudioParameterControllerInterface|SetTriggerParameter (Variables|Default|GetMS_PlayerNarrative) "Dampen")
  (Development|PrintString "Dampen"))

(fn QueueAudio
  (params (Sound%20Name :type Name))
  (Utilities|Array|Add (Variables|Sound|GetAudio%20Queue) Sound%20Name))

(fn ClearAudioQueue
  (Utilities|Array|Clear (Variables|Sound|GetAudio%20Queue)))

(fn OnNarrativeAudioFinished
  (Variables|Sound|SetIs%20Audio%20Playing false)
  (Variables|/Game/Blueprints/BP_GameInstance.BP_GameInstance_C|SetTime%20Of%20Last%20Narrative%20Sound%20End (Variables|State|GetBP%20Game%20Instance) (Utilities|Time|GetRealTimeSeconds)))