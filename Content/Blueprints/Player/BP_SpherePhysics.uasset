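; Player-controlled physics sphere that moves by force from the P1 input axes and is drawn toward nearby actors.
; Each tick it applies movement force, plus a cohesion force toward the stored other sphere while Pull is set.
; Overlaps on two triggers toggle Pull: on inside the cohesion trigger, off inside the separation trigger, with debug prints.
; A separation push force exists but is disconnected, so it never runs.
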(event OnComponentBeginOverlap(CohesionTrigger)
  (params (OverlappedComponent :type Primitive%20Component%20Object%20Reference) (OtherActor :type Actor%20Object%20Reference) (OtherComp :type Primitive%20Component%20Object%20Reference) (OtherBodyIndex :type Integer) (bFromSweep :type Boolean) (SweepResult :type Hit%20Result%20Structure%20%28by%20ref%29))
  ;[1 1 1] Start pulling
  (if (not (== OtherActor (Variables|Default|GetSeparationTrigger)))
    (bind _output_get (Variables|Default|SetOtherSphere OtherActor))
    (Variables|Default|SetbPull true)
    (Development|PrintString (Utilities|GetDisplayName _output_get))
    (Development|PrintString "Start pulling")))

(event OnComponentEndOverlap(CohesionTrigger)
  (params (OverlappedComponent :type Primitive%20Component%20Object%20Reference) (OtherActor :type Actor%20Object%20Reference) (OtherComp :type Primitive%20Component%20Object%20Reference) (OtherBodyIndex :type Integer))
  ;[1 1 1] Stop pulling
  (if (not (== OtherActor (Variables|Default|GetSeparationTrigger)))
    (Variables|Default|SetbPull false)
    (Development|PrintString "Stop pulling")))

(event OnComponentBeginOverlap(SeparationTrigger)
  (params (OverlappedComponent :type Primitive%20Component%20Object%20Reference) (OtherActor :type Actor%20Object%20Reference) (OtherComp :type Primitive%20Component%20Object%20Reference) (OtherBodyIndex :type Integer) (bFromSweep :type Boolean) (SweepResult :type Hit%20Result%20Structure%20%28by%20ref%29))
  ;[1 1 1] Start pushing
  (if (not (== OtherActor (Variables|Default|GetCohesionTrigger)))
    (bind _output_get (Variables|Default|SetOtherSphere OtherActor))
    (Variables|Default|SetbPull false)
    (Development|PrintString (Utilities|GetDisplayName _output_get))
    (Development|PrintString "Stop pulling")))

(event OnComponentEndOverlap(SeparationTrigger)
  (params (OverlappedComponent :type Primitive%20Component%20Object%20Reference) (OtherActor :type Actor%20Object%20Reference) (OtherComp :type Primitive%20Component%20Object%20Reference) (OtherBodyIndex :type Integer))
  ;[1 1 1] Stop pushing
  (if (not (== OtherActor (Variables|Default|GetCohesionTrigger)))
    (Variables|Default|SetbPull true)
    (Development|PrintString "Start pulling")))

(event EventTick
  (params (DeltaSeconds :type Float%20%28single-precision%29))
  (bind _sphere (Variables|Default|GetSphere))
  ;[1 1 1] Move in response to player input
  (Physics|AddForce (Variables|Default|GetSphere) (* (Math|Vector|Normalize (Math|Vector|MakeVector (Input|AxisValues|GetP1_UpDown) (Input|AxisValues|GetP1_RightLeft) 0.0)) (Variables|Default|GetSpeed)) "None" false)
  ;[1 1 1] Pull (if close, move towards other sphere)
  (if (Variables|Default|GetbPull)
    (Physics|AddForce _sphere (* (Math|Vector|Normalize (- (Transformation|GetActorLocation (Variables|Default|GetOtherSphere)) (Transformation|GetWorldLocation _sphere))) (Variables|Default|GetCohesionForce)) "None" false)))

(fn ConstructionScript)