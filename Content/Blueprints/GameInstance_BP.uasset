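; Game instance that holds shared state for the players: engaged flags and two-value inputs for Players A, B and C.
; Setup caches all Player_BP actors in AllPlayers, which GetActivePlayersCount loops over to count those not dead.
; A debug routine prints each player's engagement and input under a header, but its call in the event graph is never run.
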(fn PrintGameState
  (Development|PrintString (Debug|GetPlayerCStateString))
  (Development|PrintString (Debug|GetPlayerBStateString))
  (Development|PrintString (Debug|GetPlayerAStateString))
  (Development|PrintString "[ GAME INPUT STATE ]"))

(fn GetPlayerAStateString
  (bind _player_a_input (Variables|Data|GetPlayer%20A%20Input))
  (return (Utilities|String|Append "PLAYER A Engaged: " (Utilities|String|ToString(Boolean) (Variables|Data|GetPlayer%20A%20is%20Engaged)) ";  Input: " (Utilities|String|ToString(Float) (Utilities|Array|Get(acopy) _player_a_input)) ", " (Utilities|String|ToString(Float) (Utilities|Array|Get(acopy) _player_a_input 1)))))

(fn GetPlayerBStateString
  (bind _player_b_input (Variables|Data|GetPlayer%20B%20Input))
  (return (Utilities|String|Append "PLAYER B Engaged: " (Utilities|String|ToString(Boolean) (Variables|Data|GetPlayer%20B%20is%20Engaged)) ";  Input: " (Utilities|String|ToString(Float) (Utilities|Array|Get(acopy) _player_b_input)) ", " (Utilities|String|ToString(Float) (Utilities|Array|Get(acopy) _player_b_input 1)))))

(fn GetPlayerCStateString
  (bind _player_c_input (Variables|Data|GetPlayer%20C%20Input))
  (return (Utilities|String|Append "PLAYER C Engaged: " (Utilities|String|ToString(Boolean) (Variables|Data|GetPlayer%20C%20is%20Engaged)) ";  Input: " (Utilities|String|ToString(Float) (Utilities|Array|Get(acopy) _player_c_input)) ", " (Utilities|String|ToString(Float) (Utilities|Array|Get(acopy) _player_c_input 1)))))

(fn GetActivePlayersCount
  (for _array_element (Variables|State|GetAll%20Players)
    (if (not (Variables|/Game/Blueprints/Player_BP.Player_BP_C|GetIs%20Dead _array_element))
      (LocalVariables|SetActive%20Player%20Count (+ (LocalVariables|GetActive%20Player%20Count) 1))))
  (return (LocalVariables|GetActive%20Player%20Count)))

(fn Setup
  (Setup|InitializePlayers))

(fn InitializePlayers
  (bind _outactors (Actor|GetAllActorsOfClass "/Game/Blueprints/Player_BP.Player_BP_C"))
  (Variables|State|SetAll%20Players _outactors))