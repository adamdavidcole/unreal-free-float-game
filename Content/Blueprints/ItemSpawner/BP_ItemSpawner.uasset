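; Item spawner that scatters random, randomly scaled items just outside the camera's view bounds.
; An externally called Update rolls a spawn chance while players are active, picking a point beyond a random view edge.
; Each Update also destroys the oldest off-screen item once the tracked list exceeds its cap.
; A bulk off-screen cleanup exists; SpawnTrail is disconnected and unfinished, with a zero offset stacking its items.
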(event EventBeginPlay)

(fn ConstructionScript)

(fn FindIndexOfOldestActorOutOfBounds
  (for (_array_element _array_index) (Variables|ObjectsRefs|GetSpawned%20Items)
    (if (not (Default|IsPositioninBoxBounds (Variables|ObjectsRefs|GetBP%20Game%20Instance) (Default|GetViewBounds (Variables|ObjectsRefs|GetCamera)) (Transformation|GetActorLocation _array_element) 1e+02))
      (return _array_index)))
  (return -1))

(fn GetRandomItemtoSpawn
  (return (Utilities|Array|Get(acopy) (Variables|ObjectsRefs|GetItemsToSpawn) (Math|Random|RandomIntegerinRange 0 (- (Utilities|Array|Length (Variables|ObjectsRefs|GetItemsToSpawn)) 1)))))

(fn Initialize
  (Development|PrintString "Item Spawner Initialized"))

(fn GetRandomSpawnLocation
  (bind _camera (Variables|ObjectsRefs|GetCamera))
  (bind _bounds (Default|GetViewBounds _camera))
  (LocalVariables|SetOn%20Positive%20Side? (> (Math|Random|RandomFloat) 0.5))
  (if (> (Math|Random|RandomFloat) 0.5)
    (LocalVariables|SetSpawn%20Location (Utilities|GetRandomSpawnPositiononAxis (.x (.origin _bounds)) (.x (.boxextent _bounds)) (.y (.origin _bounds)) (.y (.boxextent _bounds)) (LocalVariables|GetOn%20Positive%20Side?)))
    (else
      (LocalVariables|SetSpawn%20Location (Math|Vector|MakeVector (.y (Utilities|GetRandomSpawnPositiononAxis (.y (.origin _bounds)) (.y (.boxextent _bounds)) (.x (.origin _bounds)) (.x (.boxextent _bounds)) (LocalVariables|GetOn%20Positive%20Side?))) (.x (Utilities|GetRandomSpawnPositiononAxis (.y (.origin _bounds)) (.y (.boxextent _bounds)) (.x (.origin _bounds)) (.x (.boxextent _bounds)) (LocalVariables|GetOn%20Positive%20Side?))) 0.0))))
  (return (LocalVariables|GetSpawn%20Location)))

(fn GetRandomSpawnPositiononAxis
  (params (axis%20A%20origin :type Float%20%28double-precision%29) (Axis%20A%20extent :type Float%20%28double-precision%29) (Axis%20B%20origin :type Float%20%28double-precision%29) (Axis%20B%20extent :type Float%20%28double-precision%29) (On%20Positive%20Side? :type Boolean))
  (bind _spawn_distance_overshoot_factor (Variables|Settings|GetSpawn%20Distance%20Overshoot%20Factor))
  (bind _returnvalue (* Axis%20B%20extent _spawn_distance_overshoot_factor))
  (return (Math|Vector|MakeVector (Utilities|GetRandomDistancefromAxisBounds axis%20A%20origin Axis%20A%20extent On%20Positive%20Side?) (Math|Random|RandomFloatinRange (+ Axis%20B%20origin (* _returnvalue -1.0)) (+ Axis%20B%20origin _returnvalue)) 0.0)))

(fn GetRandomDistancefromAxisBounds
  (params (Axis%20Origin :type Float%20%28double-precision%29) (Axis%20Extent :type Float%20%28double-precision%29) (On%20Positive%20Side? :type Boolean))
  (bind _max_distance_from_edge_to_spawn (Variables|Settings|GetMax%20Distance%20From%20Edge%20To%20Spawn))
  (bind _min_distance_from_edge_to_spawn (Variables|Settings|GetMin%20Distance%20From%20Edge%20To%20Spawn))
  (bind _returnvalue (Math|Random|RandomFloatinRange _min_distance_from_edge_to_spawn _max_distance_from_edge_to_spawn))
  (bind _returnvalue_2 (+ Axis%20Extent _returnvalue))
  (if On%20Positive%20Side?
    (LocalVariables|SetDistance%20from%20Origin _returnvalue_2)
    (else
      (LocalVariables|SetDistance%20from%20Origin (* _returnvalue_2 -1.0))))
  (return (+ Axis%20Origin (LocalVariables|GetDistance%20from%20Origin))))

(fn Update
  (params (Active%20Player%20Count :type Integer))
  (UpdateFuncs|MaybeSpawn Active%20Player%20Count)
  (UpdateFuncs|CleanupSingle))

(fn SpawnItem
  (params (Item%20Class :type BP%20Base%20Item%20Class%20Reference) (Location :type Vector))
  (bind _returnvalue (Math|Random|RandomFloatinRange 1.0 3.0))
  (bind _returnvalue_2 (Game|SpawnActorfromClass Item%20Class (Math|Transform|MakeTransform Location "0, 0, 0" (Math|Vector|MakeVector _returnvalue _returnvalue _returnvalue)) "AdjustIfPossibleButAlwaysSpawn" self 0))
  (Utilities|Array|Add (Variables|ObjectsRefs|GetSpawned%20Items) _returnvalue_2))

(fn MaybeSpawn
  (params (Active%20Player%20Count :type Integer))
  (if (> Active%20Player%20Count 0)
    (if (> (Variables|Settings|GetSpawn%20Probability) (Math|Random|RandomFloat))
      (UpdateFuncs|SpawnItem (Utilities|GetRandomItemtoSpawn) (Utilities|GetRandomSpawnLocation)))))

(fn FindandDestroyItem
  (params (Item :type BP%20Base%20Item%20Object%20Reference))
  (UpdateFuncs|DestroySpawnedItematIndex (Utilities|Array|FindItem (Variables|ObjectsRefs|GetSpawned%20Items) Item)))

(fn DestroySpawnedItematIndex
  (params (Index :type Integer))
  (if (or (< Index 0) (> Index (Utilities|Array|Length (Variables|ObjectsRefs|GetSpawned%20Items))))
    ;[1 1 1] Out of bounds
    (return)
    (else
      (Actor|DestroyActor (Utilities|Array|Get(acopy) (Variables|ObjectsRefs|GetSpawned%20Items) Index))
      (Utilities|Array|RemoveIndex (Variables|ObjectsRefs|GetSpawned%20Items) Index))))

(fn CleanupSingle
  (bind _index (Utilities|FindIndexOfOldestActorOutOfBounds))
  (if (> (Utilities|Array|Length (Variables|ObjectsRefs|GetSpawned%20Items)) (Variables|Settings|GetMax%20Spawn%20Count))
    (if (>= _index 0)
      (UpdateFuncs|DestroySpawnedItematIndex _index))))

(fn CleanupAllOutOfBounds
  (bind (_arrayindex _arrayelement) (Utilities|Array|ReverseforEachLoop (Variables|ObjectsRefs|GetSpawned%20Items))
    (:LoopBody
      (if (not (Default|IsPositioninBoxBounds (Variables|ObjectsRefs|GetBP%20Game%20Instance) (Default|GetViewBounds (Variables|ObjectsRefs|GetCamera)) (Transformation|GetActorLocation _arrayelement) 1e+02))
        (UpdateFuncs|DestroySpawnedItematIndex _arrayindex)))))

(fn SpawnTrail
  (bind _returnvalue (Math|Random|RandomUnitVector))
  (bind _camera (Variables|ObjectsRefs|GetCamera))
  (bind _returnvalue_2 (Transformation|GetActorLocation _camera))
  (LocalVariables|SetSpawn%20Item%20Class (Utilities|GetRandomItemtoSpawn))
  (bind _output_get (LocalVariables|SetSpawn%20Trail%20Start (Utilities|GetRandomSpawnLocation)))
  (bind _output_get_2 (LocalVariables|SetSpawn%20Trail%20Direction (Math|Vector|MakeVector (- (.x _output_get) (.x _returnvalue_2)) (- (.y _output_get) (.y _returnvalue_2)) 0.0)))
  (LocalVariables|SetSpawn%20Trail%20Direction (Math|Vector|MakeVector (.x _returnvalue) (.y _returnvalue) 0.0))
  (for _index (range 0 (LocalVariables|GetSpawn%20Trail%20Count))
    (bind _output_get_3 (LocalVariables|SetNext%20Spawn%20Location (+ (LocalVariables|GetSpawn%20Trail%20Start) (* "" _index (LocalVariables|GetSpawn%20Item%20Distance)))))
    (UpdateFuncs|SpawnItem (LocalVariables|GetSpawn%20Item%20Class) _output_get_3)
    (Development|PrintString (Utilities|String|ToString(Vector) _output_get_3))))