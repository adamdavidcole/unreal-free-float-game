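; Base item actor that a player picks up by overlapping it, with its removal handled by the item spawner that owns it.
; On BeginPlay it casts its owner to BP_ItemSpawner and caches the reference.
; Overlap with a BP_Player prints a placeholder "Hello" and calls DestroySelf, which passes the item to the spawner's FindAndDestroyItem rather than destroying it directly.
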(event EventBeginPlay
  (bind _asbp_item_spawner (Utilities|Casting|CastToBP_ItemSpawner (Components|GetOwner)))
  (Variables|Default|SetItem%20Spawner _asbp_item_spawner))

(event Collision|EventActorBeginOverlap
  (params (OtherActor :type Actor%20Object%20Reference))
  (Utilities|Casting|CastToBP_Player OtherActor)
  (Development|PrintString "Hello")
  (CallFunction|DestroySelf))

(event EventTick
  (params (DeltaSeconds :type Float%20%28single-precision%29)))

(fn ConstructionScript)

(fn DestroySelf
  (Default|FindandDestroyItem (Variables|Default|GetItem%20Spawner) self))