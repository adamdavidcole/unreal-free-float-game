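; OSC bridge that feeds external input for three players into the game.
; On BeginPlay it caches BP_GameInstance and creates a localhost OSC server and client, stored in variables to avoid garbage collection.
; Each received message is read by argument index into the game instance's engaged flags, input arrays and player states, via an int-to-enum helper.
; X and Z keys send test strings to /unreal/; the address-pattern debug listener is never executed.
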(event Custom|OnMsgReceived
  (params (Message :type OSC%20Message%20Structure%20%28by%20ref%29) (IPAddress :type String) (Port :type Integer))
  (bind _mygameinstance (Variables|Default|GetMyGameInstance))
  (bind _mygameinstance_2 (Variables|Default|GetMyGameInstance))
  (bind _mygameinstance_3 (Variables|Default|GetMyGameInstance))
  (bind _mygameinstance_4 (Variables|Default|GetMyGameInstance))
  (bind _player_b_input (Variables|/Game/Blueprints/BP_GameInstance.BP_GameInstance_C|GetPlayer%20B%20Input _mygameinstance_2))
  (bind _player_c_input (Variables|/Game/Blueprints/BP_GameInstance.BP_GameInstance_C|GetPlayer%20C%20Input _mygameinstance))
  (bind _player_a_input (Variables|/Game/Blueprints/BP_GameInstance.BP_GameInstance_C|GetPlayer%20A%20Input _mygameinstance_4))
  ;[1 1 1] Setting up to send and receive OSC messages
  ;;[1 0.3282 0] Setup to Receive Messages
  (Utilities|FlowControl|Sequence
    (:then_0
      ;;[1 1 1] Player A
      (bind (_value _returnvalue) (Class|OSCManager|GetBool Message))
      (if _returnvalue
        (Variables|/Game/Blueprints/BP_GameInstance.BP_GameInstance_C|SetPlayer%20A%20is%20Engaged _mygameinstance_4 _value)))
    (:then_1
      (bind (_value_2 _returnvalue_2) (Class|OSCManager|GetFloat Message 1))
      (if _returnvalue_2
        (Utilities|Array|SetArrayElem _player_a_input 0 _value_2)))
    (:then_2
      (bind (_value_3 _returnvalue_3) (Class|OSCManager|GetFloat Message 2))
      (if _returnvalue_3
        (Utilities|Array|SetArrayElem _player_a_input 1 _value_3)))
    (:then_3
      ;;[1 1 1] Player B
      (bind (_value_4 _returnvalue_4) (Class|OSCManager|GetBool Message 3))
      (if _returnvalue_4
        (Variables|/Game/Blueprints/BP_GameInstance.BP_GameInstance_C|SetPlayer%20B%20is%20Engaged _mygameinstance_2 _value_4)))
    (:then_4
      (bind (_value_5 _returnvalue_5) (Class|OSCManager|GetFloat Message 4))
      (if _returnvalue_5
        (Utilities|Array|SetArrayElem _player_b_input 0 _value_5)))
    (:then_5
      (bind (_value_6 _returnvalue_6) (Class|OSCManager|GetFloat Message 5))
      (if _returnvalue_6
        (Utilities|Array|SetArrayElem _player_b_input 1 _value_6)))
    (:then_6
      ;;[1 1 1] Player C
      (bind (_value_7 _returnvalue_7) (Class|OSCManager|GetBool Message 6))
      (if _returnvalue_7
        (Variables|/Game/Blueprints/BP_GameInstance.BP_GameInstance_C|SetPlayer%20C%20is%20Engaged _mygameinstance _value_7)))
    (:then_7
      (bind (_value_8 _returnvalue_8) (Class|OSCManager|GetFloat Message 7))
      (if _returnvalue_8
        (Utilities|Array|SetArrayElem _player_c_input 0 _value_8)))
    (:then_8
      (bind (_value_9 _returnvalue_9) (Class|OSCManager|GetFloat Message 8))
      (if _returnvalue_9
        (Utilities|Array|SetArrayElem _player_c_input 1 _value_9)))
    (:then_9
      ;;[1 1 1] Player State Upade
      (bind (_value_10 _returnvalue_10) (Class|OSCManager|GetInt32 Message 9))
      (if _returnvalue_10
        (Variables|/Game/Blueprints/BP_GameInstance.BP_GameInstance_C|SetPlayer%20A%20State _mygameinstance_3 (CallFunction|GetPlayerStatefromOSC _value_10))))
    (:then_10
      (bind (_value_11 _returnvalue_11) (Class|OSCManager|GetInt32 Message 10))
      (if _returnvalue_11
        (Variables|/Game/Blueprints/BP_GameInstance.BP_GameInstance_C|SetPlayer%20B%20State _mygameinstance_3 (CallFunction|GetPlayerStatefromOSC _value_11))))
    (:then_11
      (bind (_value_12 _returnvalue_12) (Class|OSCManager|GetInt32 Message 11))
      (if _returnvalue_12
        (Variables|/Game/Blueprints/BP_GameInstance.BP_GameInstance_C|SetPlayer%20C%20State _mygameinstance_3 (CallFunction|GetPlayerStatefromOSC _value_12))))))

(event Custom|OnMsgReceived_AddressPattern
  (params (AddressPattern :type OSC%20Address%20Structure%20%28by%20ref%29) (Message :type OSC%20Message%20Structure%20%28by%20ref%29) (IPAddress :type String) (Port :type Integer))
  ;[1 1 1] Binding to Address Pattern "/foo?1/slider*"
  (bind _returnvalue (Class|OSCManager|GetOSCMessageAddress Message))
  (bind _returnvalue_2 (Class|OSCManager|GetOSCAddressFullPath _returnvalue))
  (bind _value (Class|OSCManager|GetInt32 Message))
  (Development|PrintString (Utilities|String|Append "Address: " _returnvalue_2 "Value: " (Utilities|String|ToString(Integer) _value))))

(event EventBeginPlay
  ;[1 1 1] Setting up to send and receive OSC messages
  (Utilities|FlowControl|Sequence
    (:then_0
      (bind _asbp_game_instance (Utilities|Casting|CastToBP_GameInstance (Game|GetGameInstance)))
      (Variables|Default|SetMyGameInstance _asbp_game_instance))
    (:then_1
      ;;[1 0.3282 0] Setup to Receive Messages
      (bind _returnvalue (Class|OSCManager|CreateOSCServer "127.0.0.1" 8000 false true "" 0))
      ;;;[0.3356 0.4595 1] Saving as variable stops random disconnects from garbage collection
      (bind _output_get (Variables|Default|SetOSC%20Server _returnvalue))
      (EventDispatchers|AssignOnOscMessageReceived _output_get (delegate Custom|OnMsgReceived)))
    (:then_2
      ;;[0.0226 1 0] Setup to Send Messages
      (bind _returnvalue_2 (Class|OSCManager|CreateOSCClient "127.0.0.1" 12000 "Outgoing" 0))
      (Variables|Default|SetOSC%20Client _returnvalue_2)
      (bind _returnvalue_3 (Class|OSCManager|ConvertStringtoOSCAddress "/unreal/"))
      (Variables|Default|SetSendAddress _returnvalue_3))))

(event Input|KeyboardEvents|Z
  (params (Key :type Key%20Structure :default "None"))
  (:Pressed
    (bind _returnvalue (Class|OSCManager|SetOSCMessageAddress (Utilities|Struct|MakeOSCMessage) (Variables|Default|GetSendAddress)))
    (bind _returnvalue_2 (Class|OSCManager|AddString _returnvalue (Utilities|String|Append "0" "")))
    (bind _returnvalue_3 (Class|OSCManager|AddString _returnvalue_2 (Utilities|String|Append "hello" "")))
    (Class|OSCClient|SendOSCMessage (Variables|Default|GetOSC%20Client) _returnvalue_3)))

(event Input|KeyboardEvents|X
  (params (Key :type Key%20Structure :default "None"))
  ;[1 1 1] Making and sending a message
  (:Pressed
    (bind _returnvalue (Class|OSCManager|SetOSCMessageAddress (Utilities|Struct|MakeOSCMessage) (Variables|Default|GetSendAddress)))
    (bind _returnvalue_2 (Class|OSCManager|AddString _returnvalue (Utilities|String|Append "1" "")))
    (Class|OSCClient|SendOSCMessage (Variables|Default|GetOSC%20Client) _returnvalue_2)))

(fn ConstructionScript)

(fn GetPlayerStatefromOSC
  (params (OSC%20Message :type Integer))
  (switch int OSC%20Message
    (:Default
      (return "NewEnumerator0"))
    (:0
      (return "NewEnumerator0"))
    (:1
      (return "NewEnumerator1"))
    (:2
      (return "NewEnumerator2"))
    (:3
      (return "NewEnumerator3"))))