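; Player sphere pawn with a per-index colour, spawned hidden at a random location and shown on respawn near the active players.
; While active, Tick pushes the physics sphere with weighted input, alignment, cohesion and inward forces, flocking-style, then clears alignment and cohesion.
; Overlapping Trail-tagged actors destroys them and lengthens the Niagara trail.
; Boundary overlaps and a shrunken view-bounds check set the out-of-bounds flag.
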(event Custom|Event%20InitialiseMaterial
  (params (PlayerIndex :type Integer))
  (Setup|InitialiseMaterial PlayerIndex))

(event Custom|Event%20UpdateTrail
  (params (OtherActor :type Actor%20Object%20Reference))
  (Update|AbsorbTrail OtherActor))

(event EventBeginPlay
  (Variables|Default|SetbActive false)
  (bind _asbp_game_instance (Utilities|Casting|CastToBP_GameInstance (Game|GetGameInstance)))
  (Variables|Default|SetBP%20Game%20Instance _asbp_game_instance))

(event Collision|EventActorBeginOverlap
  (params (OtherActor :type Actor%20Object%20Reference))
  (Utilities|FlowControl|Sequence
    (:then_0
      (Collisions|HandleBoundaryBeginOverlap OtherActor))
    (:then_1
      (Collisions|HandleTrailBeginOverlap OtherActor))))

(event EventTick
  (params (DeltaSeconds :type Float%20%28single-precision%29))
  (if (Variables|Default|GetbActive)
    (Utilities|FlowControl|Sequence
      (:then_0
        (Update|MoveSphere))
      (:then_1
        (Update|ResetVectors)))))

(event Collision|EventActorEndOverlap
  (params (OtherActor :type Actor%20Object%20Reference))
  (Collisions|HandleBoundaryEndOverlap OtherActor))

(fn ConstructionScript)

(fn Initialize
  (params (Player%20Index :type Integer))
  (Variables|Default|SetPlayer%20Index Player%20Index)
  (Transformation|SetActorLocation (Math|Vector|MakeVector (Math|Random|RandomFloatinRange -5e+02 5e+02) (Math|Random|RandomFloatinRange -5e+02 5e+02) 0.0) false false)
  (Setup|InitialiseMaterial Player%20Index)
  (Rendering|SetActorHiddenInGame true)
  (Development|PrintString (Utilities|String|Append "Player " (Utilities|String|ToString(Integer) (Variables|Default|GetPlayer%20Index)) " spawned"))
  (Development|PrintString (Utilities|String|ToString(Vector) (Transformation|GetActorLocation)) true true "(R=0.000000,G=1.000000,B=0.134609,A=1.000000)"))

(fn InitialiseMaterial
  (params (Player%20Index :type Integer))
  (bind _returnvalue (Rendering|Material|CreateDynamicMaterialInstance (Variables|Default|GetSphere) 0 "/Game/Materials/M_Sphere.M_Sphere" "None" :!class /Script/Engine.PrimitiveComponent))
  (Rendering|Material|SetVectorParameterValue _returnvalue "Colour" (Utilities|Array|Get(acopy) (Variables|Default|GetSphereColours) Player%20Index) :!class /Script/Engine.MaterialInstanceDynamic))

(fn HandleBoundaryEndOverlap
  (params (OtherActor :type Actor%20Object%20Reference))
  (if (Actor|ActorHasTag OtherActor "Boundaries")
    (Variables|Default|SetbOutOfBounds true)))

(fn HandleTrailBeginOverlap
  (params (OtherActor :type Actor%20Object%20Reference))
  (if (Actor|ActorHasTag OtherActor "Trail")
    (CallFunction|EventUpdateTrail OtherActor)))

(fn HandleBoundaryBeginOverlap
  (params (Other%20Actor :type Actor%20Object%20Reference))
  (if (Actor|ActorHasTag Other%20Actor "Boundaries")
    (Variables|Default|SetbOutOfBounds false)
    (Development|PrintString "Hello")))

(fn UpdateOutOfBounds
  (params (View%20Bounds :type Box%20Sphere%20Bounds%20Structure))
  (Variables|Default|SetbOutOfBounds (Utilties|IsinViewBounds View%20Bounds)))

(fn AbsorbTrail
  (params (Other%20Actor :type Actor%20Object%20Reference))
  (Niagara|SetNiagaraVariable(Float) (Variables|Default|GetTrail) "User.TrailLength" (+ (Variables|Default|GetTrailLength) 0.1))
  (Variables|Default|SetTrailLength (+ (Variables|Default|GetTrailLength) 0.1))
  (Actor|DestroyActor Other%20Actor))

(fn MoveSphere
  (Physics|AddForce (Variables|Default|GetSphere) (+ (* (Variables|Default|GetInputVector) (Variables|Default|GetSpeed)) (* (Variables|Default|GetAlignmentVector) (Variables|Default|GetAlignmentWeight) (Variables|Default|GetSpeed)) (* (Variables|Default|GetCohesionVector) (Variables|Default|GetCohesionWeight) (Variables|Default|GetSpeed)) (* (Variables|Default|GetInwardForceVector) (Variables|Default|GetInwardForceWeight) (Variables|Default|GetSpeed))) "None" false))

(fn ResetVectors
  (Variables|Default|SetAlignmentVector "0, 0, 0")
  (Variables|Default|SetCohesionVector "0, 0, 0"))

(fn Respawn
  (params (Players :type Array%20of%20BP%20Player%20Object%20References))
  (Transformation|SetActorLocation (Utilties|GetRespawnLocation Players) false false)
  (Rendering|SetActorHiddenInGame false)
  (Development|PrintString (Utilities|String|Append "Player  active: " (Utilities|String|ToString(Integer) (Variables|Default|GetPlayer%20Index)))))

(fn IsinViewBounds
  (params (Bounds :type Box%20Sphere%20Bounds%20Structure))
  (bind _returnvalue (Transformation|GetActorLocation))
  (bind _bounds_shrink_factor (LocalVariables|GetBounds%20Shrink%20Factor))
  (bind _bounds_shrink_factor_2 (LocalVariables|GetBounds%20Shrink%20Factor))
  (bind _returnvalue_2 (- (.x _returnvalue) (.x (.origin Bounds))))
  (bind _returnvalue_3 (* (.x (.boxextent Bounds)) _bounds_shrink_factor_2))
  (bind _returnvalue_4 (* (.y (.boxextent Bounds)) _bounds_shrink_factor))
  (bind _returnvalue_5 (- (.y _returnvalue) (.y (.origin Bounds))))
  (bind _returnvalue_6 (Math|Float|Absolute(Float) _returnvalue_5))
  (bind _returnvalue_7 (Math|Float|Absolute(Float) _returnvalue_2))
  (bind _returnvalue_8 (> _returnvalue_7 _returnvalue_3))
  (bind _returnvalue_9 (> _returnvalue_6 _returnvalue_4))
  (bind _returnvalue_10 (or _returnvalue_8 _returnvalue_9))
  (if _returnvalue_10
    (Development|PrintString (Utilities|String|Append "Player Out of Bounds: " (Utilities|String|ToString(Integer) (Variables|Default|GetPlayer%20Index))))
    (return _returnvalue_10)))

(fn Die
  (Rendering|SetActorHiddenInGame true)
  (Development|PrintString (Utilities|String|Append "Player  inactive: " (Utilities|String|ToString(Integer) (Variables|Default|GetPlayer%20Index)))))

(fn GetRespawnLocation
  (params (Players :type Array%20of%20BP%20Player%20Object%20References))
  (bind _returnvalue (Math|Random|RandomUnitVector))
  (bind _min_spawn_distance (LocalVariables|GetMin%20Spawn%20Distance))
  (bind _max_spawn_distance (LocalVariables|GetMax%20Spawn%20Distance))
  (bind _returnvalue_2 (Math|Random|RandomFloatinRange _min_spawn_distance _max_spawn_distance))
  (bind _returnvalue_3 (* _returnvalue _returnvalue_2))
  (bind _center (Collision|GetActorArrayBounds (Default|GetActivePlayers (Variables|Default|GetBP%20Game%20Instance) Players) true))
  (return (+ _center (Math|Vector|MakeVector (.x _returnvalue_3) (.y _returnvalue_3) 0.0))))